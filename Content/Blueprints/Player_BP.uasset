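; Player character for a 2D side-scroller, with running, jumping, wall jumping, dashing, climbing and projectile shooting.
; Input events drive movement: a line trace finds walls to kick off, dash launches along current velocity, and climbing uses Flying mode while CanClimb is set.
; Each tick flips the sprite by X velocity and picks its flipbook through a priority-ordered state function.
; Jumps and landings spawn dust and squash-and-stretch the actor through timelines.
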(event `self.ReceiveTick`
  (params (DeltaSeconds :type "Float (single-precision)"))
  ;[1 1 1] Update
  ;;[1 1 1] Tick
  (`self.UpdateAnimation`)
  ;;[1 1 1] Flip sprite based on axis
  (`/Engine/EditorBlueprintResources/StandardMacros.CompareFloat` (.x (`MovementComponent.Velocity` (`self.CharacterMovement`)))
    (:`>`
      (`SceneComponent.K2_SetRelativeRotation` :`self` (`self.Sprite`)))
    (:`<`
      (`SceneComponent.K2_SetRelativeRotation` (`self.Sprite`) (struct :`Yaw` 180.0) false false))))

(event `InputAction|Jump`
  (params (Key :type "Key Structure"))
  ;[1 1 1] Jumping
  (:`Pressed`
    (`PaperFlipbookComponent.SetFlipbook` (`self.Sprite`) "/Game/Art/Sprites/Character/Grey_Jump.Grey_Jump")
    (if (`NavMovementComponent.IsFalling` (`self.CharacterMovement`))
      (`self.WallJump`)
      (else
        (`self.Jump`)
        (`self.JumpFX`))))
  (:`Released`
    (`self.StopJumping`)))

(event `InputAxis|Right`
  (params (AxisValue :type "Float (single-precision)"))
  ;[1 1 1] Movement Control
  (`self.AddMovementInput` (1.0 0.0 0.0) AxisValue))

(event `self.OnLanded`
  (params (Hit :type "HitResult Structure (by ref)"))
  ;[1 1 1] Landed
  (`self.LandFX`))

(event `WallJump`
  (bind _returnvalue (`self.GetActorForwardVector`))
  (bind _returnvalue_x (`KismetMathLibrary.BreakVector` (`self.K2_GetActorLocation`)))
  ;[1 1 1] Wall Jump
  (bind (_outhit _returnvalue_2) (`KismetSystemLibrary.LineTraceSingle` :`Start` (- (`self.K2_GetActorLocation`) (* _returnvalue (+ (`CapsuleComponent.GetScaledCapsuleRadius` (`self.CapsuleComponent`)) 15.0))) :`End` (+ (`self.K2_GetActorLocation`) (* _returnvalue (+ (`CapsuleComponent.GetScaledCapsuleRadius` (`self.CapsuleComponent`)) 15.0))) :`TraceChannel` "TraceTypeQuery1" :`bTraceComplex` true :`DrawDebugType` "Persistent"))
  (if _returnvalue_2
    (`self.LaunchCharacter` (`KismetMathLibrary.MakeVector` (* (`KismetMathLibrary.SignOfFloat` (- _returnvalue_x (.x (`.Location` (`GameplayStatics.BreakHitResult` _outhit))))) 450.0) 0.0 (`CharacterMovementComponent.JumpZVelocity` (`self.CharacterMovement`))) true true)
    (`self.JumpFX`)
    (elif (< (`self.JumpCurrentCount`) (`self.JumpMaxCount`))
      (`self.Jump`)
      (`self.JumpFX`))))

(event `InputAction|Dash`
  (params (Key :type "Key Structure"))
  (bind _returnvalue (`self.GetVelocity`))
  ;[1 1 1] Dash
  (:`Pressed`
    (if (!= _returnvalue (0.0 0.0 0.0))
      (if (`NavMovementComponent.IsFalling` (`self.CharacterMovement`))
        (`self.LaunchCharacter` (* (+ _returnvalue (0.0 0.0 0.0)) (1.5 1.5 1.5)) true true)
        (else
          (`self.LaunchCharacter` (* (+ _returnvalue (0.0 0.0 1.0)) (1.5 1.5 250.0))))))))

(event `JumpFX`
  ;[1 1 1] Jump Effects
  (`GameplayStatics.SpawnEmitterAtLocation` "/Game/Art/Particles/P_dust.P_dust" (`SceneComponent.K2_GetComponentLocation` (`self.DustBox`)))
  (bind (_direction _squash) (`Timeline|Timeline_0` :!via `PlayFromStart`)
    (:`Update`
      (`self.SetActorScale3D` (`KismetMathLibrary.VLerp` (1.0 1.0 1.0) (0.5 1.0 1.5) _squash)))))

(event `LandFX`
  ;[1 1 1] Jump Effects
  (`GameplayStatics.SpawnEmitterAtLocation` "/Game/Art/Particles/P_dust.P_dust" (`SceneComponent.K2_GetComponentLocation` (`self.DustBox`)))
  (bind (_direction _squash) (`Timeline|Timeline_1` :!via `PlayFromStart`)
    (:`Update`
      (`self.SetActorScale3D` (`KismetMathLibrary.VLerp` (1.0 1.0 1.0) (1.5 1.0 0.5) _squash)))))

(event `UpdateAnimation`
  ;[1 1 1] Control Animations
  (set `self.IsMoving` (> (`KismetMathLibrary.VSize` (`self.GetVelocity`)) 0.0))
  (bind _outputfb (`self.AnimationStateMachine` (`self.IsMoving`) (`NavMovementComponent.IsFalling` (`self.CharacterMovement`)) (`self.IsDashing`) (`self.IsAttacking`) (`self.IsClimbing`)))
  (`PaperFlipbookComponent.SetFlipbook` (`self.Sprite`) _outputfb))

(event `InputAction|Shoot`
  (params (Key :type "Key Structure"))
  ;[1 1 1] Attacking
  (:`Pressed`
    (if (not (`self.IsAttacking`))
      (`self.AttackAnimation`))))

(event `FireProjectile`
  ;[1 1 1] Attacking
  (`|SpawnActorFromClass` "/Game/Blueprints/projectile_BP.projectile_BP_C" (`SceneComponent.K2_GetComponentToWorld` (`self.ProjectileSpawn`)) "AlwaysSpawn" "OverrideRootScale" null null))

(event `AttackAnimation`
  ;[1 1 1] Attacking
  (`|ExecutionSequence`
    (:`then_0`
      (set `self.IsAttacking` true)
      (`self.FireProjectile`))
    (:`then_1`
      (`KismetSystemLibrary.Delay` (/ 2.0 (`PaperFlipbook.FramesPerSecond` (`self.AttackingFB`))))
      (set `self.IsAttacking` false))))

(event `InputAxis|MoveUp`
  (params (AxisValue :type "Float (single-precision)"))
  (if (`self.CanClimb`)
    (if (`KismetMathLibrary.InRange_FloatFloat` AxisValue -0.1 0.1)
      (`PaperFlipbookComponent.SetPlayRate` (`self.Sprite`) 0.0)
      (else
        (set `self.IsClimbing` true)
        (`PaperFlipbookComponent.SetPlayRate` (`self.Sprite`) 1.0)
        (`CharacterMovementComponent.SetMovementMode` (`self.CharacterMovement`) "MOVE_Flying" 0)
        (`self.AddMovementInput` (0.0 0.0 0.5) AxisValue)))))

(event `ClimbingEnd`
  (`CharacterMovementComponent.SetMovementMode` (`self.CharacterMovement`) "MOVE_Walking" 0)
  (set `self.IsClimbing` false)
  (`PaperFlipbookComponent.SetPlayRate` (`self.Sprite`) 1.0))

(fn `AnimationStateMachine`
  (params (IsMoving :type Boolean) (IsFalling :type Boolean) (IsDashing :type Boolean) (IsAttacking :type Boolean) (IsClimbing :type Boolean))
  (returns (OutputFB :type "PaperFlipbook Object Reference"))
  (locals (AnimationState :type "/Game/Data/AnimationState Enum" :default "NewEnumerator0"))
  (if IsClimbing
    (set `local.AnimationState` "NewEnumerator5")
    (elif IsDashing
      (set `local.AnimationState` "NewEnumerator3")
      (elif IsAttacking
        (set `local.AnimationState` "NewEnumerator4")
        (elif IsFalling
          (set `local.AnimationState` "NewEnumerator2")
          (elif IsMoving
            (set `local.AnimationState` "NewEnumerator1")
            (else
              (set `local.AnimationState` "NewEnumerator0")))))))
  (return (select `/Game/Data/AnimationState` (`local.AnimationState`) :`NewEnumerator0` (`self.IdleFB`) :`NewEnumerator1` (`self.RunningFB`) :`NewEnumerator2` (`self.JumpingFB`) :`NewEnumerator3` (`self.DashingFB`) :`NewEnumerator4` (`self.AttackingFB`) :`NewEnumerator5` (`self.ClimbingFB`))))

(fn `UserConstructionScript`
  (set `CharacterMovementComponent.JumpZVelocity` 400.0 (`self.CharacterMovement`))
  (set `self.JumpMaxHoldTime` 0.3))